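; BP_Log is a log actor that moves in steps and carries BP_Frog_New.
; Tick counts down a timer and calls Move every StepDelay, shifting the log along world X by Direction times StepDistance without sweep.
; Box1 overlap attaches the frog to the log, snapping its location to the attach target, and end overlap detaches it at its world location.
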(event OnComponentBeginOverlap(Box1)
  (params (OverlappedComponent :type Primitive%20Component%20Object%20Reference) (OtherActor :type Actor%20Object%20Reference) (OtherComp :type Primitive%20Component%20Object%20Reference) (OtherBodyIndex :type Integer) (bFromSweep :type Boolean) (SweepResult :type Hit%20Result%20Structure%20%28by%20ref%29))
  (bind _asbp_frog_new (Utilities|Casting|CastToBP_Frog_New OtherActor))
  (Transformation|AttachActorToActor _asbp_frog_new self "None" "SnapToTarget" "KeepRelative" "KeepRelative" true))

(event OnComponentEndOverlap(Box1)
  (params (OverlappedComponent :type Primitive%20Component%20Object%20Reference) (OtherActor :type Actor%20Object%20Reference) (OtherComp :type Primitive%20Component%20Object%20Reference) (OtherBodyIndex :type Integer))
  (bind _asbp_frog_new (Utilities|Casting|CastToBP_Frog_New OtherActor))
  (Transformation|DetachFromActor _asbp_frog_new "KeepWorld" "KeepRelative" "KeepRelative"))

(event EventBeginPlay)

(event Collision|EventActorBeginOverlap
  (params (OtherActor :type Actor%20Object%20Reference)))

(event EventTick
  (params (DeltaSeconds :type Float%20%28single-precision%29))
  (Variables|Default|Settimer (- (Variables|Default|Gettimer) DeltaSeconds))
  (if (<= (Variables|Default|Gettimer) 0.0)
    (CallFunction|Move (Variables|Default|Getdirection))
    (Variables|Default|Settimer (Variables|Default|GetstepDelay))))

(fn ConstructionScript)

(fn Move
  (params (direction :type Float%20%28double-precision%29))
  (bind _returnvalue (Transformation|GetActorLocation))
  (Transformation|SetActorLocation (Math|Vector|MakeVector (+ (* direction (Variables|Default|GetstepDistance)) (.x _returnvalue)) (.y _returnvalue) (.z _returnvalue)) false false))