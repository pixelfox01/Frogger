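; BP_Spawner is an actor that repeatedly spawns moving obstacles (cars, logs or long logs) at its own location.
; Tick counts down a timer, calls SpawnObstacle, then resets the timer to a random interval for cars or a fixed delay for other types.
; SpawnObstacle spawns the configured class and uses a cast chain to pass the spawner's direction and step delay to the new obstacle.
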(event EventBeginPlay)

(event Collision|EventActorBeginOverlap
  (params (OtherActor :type Actor%20Object%20Reference)))

(event EventTick
  (params (DeltaSeconds :type Float%20%28single-precision%29))
  (if (<= (Variables|Default|GetspawnTimer) 0.0)
    (CallFunction|SpawnObstacle)
    (if (Utilities|Enum|Equal(Enum) (Variables|Default|GetobstacleType) "car")
      (Variables|Default|SetspawnTimer (Math|Random|RandomFloatinRange 2.0 4.5))
      (else
        (Variables|Default|SetspawnTimer (Variables|Default|GetspawnDelay))))
    (else
      (Variables|Default|SetspawnTimer (- (Variables|Default|GetspawnTimer) DeltaSeconds)))))

(fn ConstructionScript)

(fn SpawnObstacle
  (bind _returnvalue (Game|SpawnActorfromClass (Variables|Default|GetobstacleBP) (Math|Conversions|ToTransform(Vector) (Transformation|GetActorLocation)) "Undefined" 0 0))
  (bind _asbp_car (Utilities|Casting|CastToBP_Car _returnvalue)
    (:then
      (Variables|/Game/Blueprints/BP_Car.BP_Car_C|Setdirection _asbp_car (Variables|Default|GetobstacleDirection))
      (Variables|/Game/Blueprints/BP_Car.BP_Car_C|SetstepDelay _asbp_car (Variables|Default|GetobstacleStepDelay)))
    (:CastFailed
      (bind _asbp_log (Utilities|Casting|CastToBP_Log _returnvalue)
        (:then
          (Variables|/Game/Blueprints/BP_Log.BP_Log_C|Setdirection _asbp_log (Variables|Default|GetobstacleDirection))
          (Variables|/Game/Blueprints/BP_Log.BP_Log_C|SetstepDelay _asbp_log (Variables|Default|GetobstacleStepDelay)))
        (:CastFailed
          (bind _asbp_log_long (Utilities|Casting|CastToBP_Log_Long _returnvalue))
          (Variables|/Game/Blueprints/BP_Log_Long.BP_Log_Long_C|Setdirection _asbp_log_long (Variables|Default|GetobstacleDirection))
          (Variables|/Game/Blueprints/BP_Log_Long.BP_Log_Long_C|SetstepDelay _asbp_log_long (Variables|Default|GetobstacleStepDelay)))))))