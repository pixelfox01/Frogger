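; BP_Frog_New is a player-controlled frog that moves in discrete steps on a flat X-Z plane.
; Right, Left, Up and Down input presses call MovePlayer with a positive or negative MoveX or MoveZ step.
; MovePlayer adds the step to the current location, clamps X and Z to fixed bounds, pins Y at zero and sets the location without sweeping.
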(event EventBeginPlay)

(event Collision|EventActorBeginOverlap
  (params (OtherActor :type Actor%20Object%20Reference)))

(event EventTick
  (params (DeltaSeconds :type Float%20%28single-precision%29)))

(event Input|ActionEvents|InputActionRight
  (params (Key :type Key%20Structure :default "None"))
  (:Pressed
    (CallFunction|MovePlayer (Variables|Default|GetmoveX) 0.0)))

(event Input|ActionEvents|InputActionLeft
  (params (Key :type Key%20Structure :default "None"))
  (:Pressed
    (CallFunction|MovePlayer (* (Variables|Default|GetmoveX) -1.0) 0.0)))

(event Input|ActionEvents|InputActionDown
  (params (Key :type Key%20Structure :default "None"))
  (:Pressed
    (CallFunction|MovePlayer 0.0 (* (Variables|Default|GetmoveZ) -1.0))))

(event Input|ActionEvents|InputActionUp
  (params (Key :type Key%20Structure :default "None"))
  (:Pressed
    (CallFunction|MovePlayer 0.0 (Variables|Default|GetmoveZ))))

(fn ConstructionScript)

(fn MovePlayer
  (params (xMove :type Float%20%28double-precision%29) (zMove :type Float%20%28double-precision%29))
  (bind _returnvalue (Transformation|GetActorLocation))
  (Transformation|SetActorLocation (Math|Vector|MakeVector (Math|Float|Clamp(Float) (+ xMove (.x _returnvalue)) 0.0 72.0) 0.0 (Math|Float|Clamp(Float) (+ zMove (.z _returnvalue)) -96.0 2.0)) false false))