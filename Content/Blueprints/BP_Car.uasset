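; BP_Car is a 2D sprite car that moves along the X axis in discrete steps.
; Shortly after BeginPlay it picks a random sprite from its Sprites array and rotates 180 degrees when Direction is positive.
; Tick counts down a timer, then calls Move to shift the location by Direction times StepDistance without sweeping, and resets the timer to StepDelay.
; The overlap event is an empty stub.
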(event EventBeginPlay
  (Utilities|FlowControl|Delay 0.2)
  (Rendering|Components|Sprite|SetSprite (Variables|Default|GetPaperSprite) (.OutItem (Utilities|Array|Random (Variables|Default|Getsprites))))
  (if (> (Variables|Default|Getdirection) 0.0)
    (Transformation|SetActorRotation "0,180.000000, 0")))

(event Collision|EventActorBeginOverlap
  (params (OtherActor :type Actor%20Object%20Reference)))

(event EventTick
  (params (DeltaSeconds :type Float%20%28single-precision%29))
  (Variables|Default|Settimer (- (Variables|Default|Gettimer) DeltaSeconds))
  (if (<= (Variables|Default|Gettimer) 0.0)
    (CallFunction|Move (Variables|Default|Getdirection))
    (Variables|Default|Settimer (Variables|Default|GetstepDelay))))

(fn ConstructionScript)

(fn Move
  (params (direction :type Float%20%28double-precision%29))
  (bind _returnvalue (Transformation|GetActorLocation))
  (Transformation|SetActorLocation (Math|Vector|MakeVector (+ (* direction (Variables|Default|GetstepDistance)) (.x _returnvalue)) (.y _returnvalue) (.z _returnvalue)) false false))